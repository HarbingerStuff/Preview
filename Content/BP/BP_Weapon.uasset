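; BP_Weapon is a mouse-aimed automatic weapon that spawns BP_Projectile actors from its Arrow component's transform.
; It enables player 0 input on BeginPlay; holding left mouse runs a looping FireRate timer calling StartFire, cleared by name on release or StopFire.
; Tick yaws the Cube toward the trace end of the under-cursor visibility trace, setting it as relative rotation with zero pitch and roll.
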(event `Start Fire`
  (`|SpawnActorFromClass` "/Game/BP/BP_Projectile.BP_Projectile_C" (`SceneComponent.K2_GetComponentToWorld` (`self.Arrow`)) "Undefined" "OverrideRootScale" null null))

(event `self.ReceiveBeginPlay`
  (`self.EnableInput` (`GameplayStatics.GetPlayerController` 0)))

(event `Key|LeftMouseButton`
  (params (Key :type "Key Structure"))
  (:`Pressed`
    (`KismetSystemLibrary.K2_SetTimerDelegate` (delegate `Start Fire`) (`self.FireRate`) true -0.0))
  (:`Released`
    (`KismetSystemLibrary.K2_ClearTimer` null "Start Fire")))

(event `Stop Fire`
  (`KismetSystemLibrary.K2_ClearTimer` null "Start Fire"))

(event `self.ReceiveTick`
  (params (DeltaSeconds :type "Float (single-precision)"))
  (bind (_returnvalue_roll _returnvalue_pitch _returnvalue_yaw) (`KismetMathLibrary.BreakRotator` (`KismetMathLibrary.FindLookAtRotation` (`SceneComponent.K2_GetComponentLocation` (`self.Cube`)) (`.TraceEnd` (`GameplayStatics.BreakHitResult` (`PlayerController.GetHitResultUnderCursorByChannel` (`GameplayStatics.GetPlayerController` 0) "TraceTypeQuery1" true))))))
  (bind (_returnvalue_roll_2 _returnvalue_pitch_2 _returnvalue_yaw_2) (`KismetMathLibrary.BreakRotator` (`KismetMathLibrary.MakeRotator` 0.0 0.0 _returnvalue_yaw)))
  (`SceneComponent.K2_SetRelativeRotation` (`self.Cube`) (`KismetMathLibrary.MakeRotator` 0.0 0.0 (`KismetMathLibrary.ClampAxis` _returnvalue_yaw_2)) false false))

(fn `UserConstructionScript`)